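; Inventory component that stores item stacks in a slot-keyed map and toggles the UMG_Inventory widget through Enhanced Input, switching cursor and input mode.
; The widget receives the map and slot settings, and its add, drop and remove events are bound on opening.
; PickUpItem scans slots for matching items and the first empty key, where leftover quantity goes.
; Dropping box-traces downward ahead of the owner and always spawns BP_Cristal at the hit.
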(event `self.ReceiveBeginPlay`
  (`EnhancedInputSubsystemInterface.AddMappingContext` (pcsubsystem `EnhancedInputLocalPlayerSubsystem` (`GameplayStatics.GetPlayerController` 0)) "/Game/Inventory/IMC_Inventory.IMC_Inventory" 0 (struct)))

(event `EnhancedInput|/Game/Inventory/IA_Inventory`
  (params (ActionValue :type Boolean) (ElapsedSeconds :type "Float (double-precision)") (TriggeredSeconds :type "Float (double-precision)") (InputAction :type "InputAction Object Reference" :default "/Game/Inventory/IA_Inventory.IA_Inventory"))
  (bind _returnvalue (`GameplayStatics.GetPlayerController` 0))
  (bind _returnvalue_2 (`GameplayStatics.GetPlayerController` 0))
  (bind _as_umg_inventory (`self.As UMG_Inventory`))
  (:`Started`
    (`self.As UMG_Inventory`
      (:`then`
        (set `PlayerController.bShowMouseCursor` false _returnvalue)
        (`WidgetBlueprintLibrary.SetInputMode_GameOnly` _returnvalue true)
        (`Widget.RemoveFromParent` (`self.As UMG_Inventory`))
        (set `self.As UMG_Inventory` null)
        (`KismetSystemLibrary.PrintString` "Inventory Closed"))
      (:`else`
        (bind _returnvalue_3 (`|CreateWidget` "/Game/Inventory/Widgets/UMG_Inventory.UMG_Inventory_C" null (`self.Inventory`) (`self.MaxSize`) (`self.AllowDuplicates`)))
        (bind _output_get (set `self.As UMG_Inventory` _returnvalue_3))
        (`UserWidget.AddToViewport` _output_get 0)
        (add `/Game/Inventory/Widgets/UMG_Inventory.ItemAdded` _as_umg_inventory (`|CreateDelegate` :!event `ItemAdded`))
        (add `/Game/Inventory/Widgets/UMG_Inventory.ItemDropped` _as_umg_inventory (`|CreateDelegate` :!event `ItemDropped`))
        (add `/Game/Inventory/Widgets/UMG_Inventory.ItemRemoved` _as_umg_inventory (`|CreateDelegate` :!event `ItemRemoved`))
        (set `PlayerController.bShowMouseCursor` true _returnvalue_2)
        (`WidgetBlueprintLibrary.SetInputMode_GameAndUIEx` _returnvalue_2 null)
        (`KismetSystemLibrary.PrintString` "Inventory Opened")))))

(fn `IsKeyFull`
  (params (Key :type Integer))
  (returns (ReturnValue :type Boolean) (Remaining :type Integer))
  (bind (_value _returnvalue) (`BlueprintMapLibrary.Map_Find` (`self.Inventory`) (`local.Key`)))
  (bind (_quantity _dataasset) (break `/Game/Inventory/Items/ST_Inventory` _value))
  (bind _maxstack (`/Game/Inventory/Items/DA_Items.MaxStack` _dataasset))
  (bind _returnvalue_2 (- _maxstack _quantity))
  (if _returnvalue
    (return (and (== _returnvalue_2 0) (!= _maxstack 0)) _returnvalue_2)
    (else
      (return false -1))))

(fn `ItemAdded`
  (params (SlotKey :type Integer) (SlotValue :type "/Game/Inventory/Items/ST_Inventory Structure"))
  (`BlueprintMapLibrary.Map_Add` (`self.Inventory`) SlotKey SlotValue))

(fn `ItemDropped`
  (params (ItemDropped :type "/Game/Inventory/Items/ST_Inventory Structure"))
  (bind _returnvalue (`self.GetOwner`))
  (bind _returnvalue_2 (+ (* (`Actor.GetActorForwardVector` _returnvalue) 300.0) (`Actor.K2_GetActorLocation` _returnvalue)))
  (bind (_outhit _returnvalue_3) (`KismetSystemLibrary.BoxTraceSingle` _returnvalue_2 (- _returnvalue_2 (0.0 0.0 500.0)) (15.0 15.0 15.0) (struct) "TraceTypeQuery1" false (`|MakeArray` (`self.GetOwner`))))
  (if _returnvalue_3
    (`|SpawnActorFromClass` "/Game/Interaction/BP_Cristal.BP_Cristal_C" (`KismetMathLibrary.MakeTransform` (`.ImpactPoint` (`GameplayStatics.BreakHitResult` _outhit))) "Undefined" "MultiplyWithRoot" null (struct) null)))

(fn `ItemRemoved`
  (params (Key :type Integer))
  (`BlueprintMapLibrary.Map_Remove` (`self.Inventory`) Key))

(fn `PickUpItem`
  (params (Item :type "/Game/Interaction/BP_Cristal Object Reference"))
  (returns (ReturnValue :type Boolean))
  (locals (`L-QuantityIn` :type Integer) (`L-dataAssetIn` :type "/Game/Inventory/Items/DA_Items Object Reference") (`L-Index` :type Integer) (`L-FoundSameItem` :type Boolean) (`L-Remaining` :type Integer :default 0) (`L-EmptyKey` :type Integer :default -1))
  (bind (_quantity _dataasset) (break `/Game/Inventory/Items/ST_Inventory` (`/Game/Interaction/BP_Cristal.Structure` Item)))
  (bind _value (`BlueprintMapLibrary.Map_Find` (`self.Inventory`) (`local.L-Index`)))
  (bind _returnvalue (- (`local.L-QuantityIn`) (`local.L-Remaining`)))
  (set `local.L-QuantityIn` _quantity)
  (set `local.L-dataAssetIn` _dataasset)
  (while (and (> (`local.L-QuantityIn`) 0) (< (`local.L-Index`) (`self.MaxSize`)))
    (`|ExecutionSequence`
      (:`then_0`
        (bind (_returnvalue_2 _remaining) (`self.IsKeyFull` (`local.L-Index`)))
        (if _returnvalue_2
          (if (== (`.DataAsset_6_EE368C1C45EA8352B6AFF6ADE8012CEC` (break `/Game/Inventory/Items/ST_Inventory` (`BlueprintMapLibrary.Map_Find` (`self.Inventory`) (`local.L-Index`)))) (`local.L-dataAssetIn`))
            (set `local.L-FoundSameItem` true))
          (else
            (bind _output_get (set `local.L-Remaining` _remaining))
            (if (== _output_get -1)
              (if (== -1 (`local.L-EmptyKey`))
                (set `local.L-EmptyKey` (`local.L-Index`))
                (elif (== (`.DataAsset_6_EE368C1C45EA8352B6AFF6ADE8012CEC` (break `/Game/Inventory/Items/ST_Inventory` _value)) (`local.L-dataAssetIn`))
                  (`BlueprintMapLibrary.Map_Add` (`self.Inventory`) (`local.L-Index`) (make `/Game/Inventory/Items/ST_Inventory` (+ (break `/Game/Inventory/Items/ST_Inventory` _value) (`KismetMathLibrary.Clamp` (`local.L-QuantityIn`) 0 (`local.L-Remaining`))) (`local.L-dataAssetIn`)))
                  (set `local.L-QuantityIn` (`KismetMathLibrary.Clamp` _returnvalue 0 _returnvalue))
                  (set `local.L-FoundSameItem` true)))))))
      (:`then_1`
        (`/Engine/EditorBlueprintResources/StandardMacros.IncrementInt` (`local.L-Index`)))))
  (if (== (`local.L-QuantityIn`) 0)
    (return true)
    (else
      (`KismetSystemLibrary.PrintString` "AAAAA")
      (if (!= (`local.L-EmptyKey`) -1)
        (`KismetSystemLibrary.PrintString` "BBBBB")
        (`BlueprintMapLibrary.Map_Add` (`self.Inventory`) (`local.L-EmptyKey`) (make `/Game/Inventory/Items/ST_Inventory` (`local.L-QuantityIn`) (`local.L-dataAssetIn`)))
        (return true)
        (else
          (`KismetSystemLibrary.PrintString` "CCCC")
          (return false))))))