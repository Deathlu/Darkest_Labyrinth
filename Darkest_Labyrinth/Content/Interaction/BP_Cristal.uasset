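; BP_Cristal is a crystal pickup that takes its mesh from a data asset, destroying itself without one.
; Sphere overlap passes it to the overlapping actor's AC_Inventory, destroying it on success.
; Interacting plays a timeline pulling it toward the camera, then InteractOnServer flips InteractToggle, whose OnRep tries pickup via an inventory component on the camera manager.
; The interaction interface also exposes a widget; focus changes only print debug text.
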(event `self.ReceiveBeginPlay`
  (bind (_quantity _dataasset) (break `/Game/Inventory/Items/ST_Inventory` (`self.Structure`)))
  (`/Engine/EditorBlueprintResources/StandardMacros.IsValid` _dataasset
    (:`Is Valid`
      (`StaticMeshComponent.SetStaticMesh` (`self.Cristall`) (`/Game/Inventory/Items/DA_Items.StaticMesh` _dataasset)))
    (:`Is Not Valid`
      (`self.K2_DestroyActor`))))

(event `/Game/Interaction/BI_Interaction.Interface_ToggleFocus`
  (params (Focus :type Boolean))
  (`KismetSystemLibrary.PrintText` (`KismetTextLibrary.Conv_BoolToText` Focus) true true (struct :`R` 1.0 :`G` 0.109375 :`B` 0.109375 :`A` 1.0)))

(event `/Game/Interaction/BI_Interaction.InterfaceInteract`
  (bind (_direction _newtrack_1) (`Timeline|MoveItem`)
    (:`Update`
      (`self.K2_SetActorLocation` (`KismetMathLibrary.VLerp` (`self.K2_GetActorLocation`) (`self.K2_GetActorLocation` (`GameplayStatics.GetPlayerCameraManager` 0)) _newtrack_1)))
    (:`Finished`
      (`self.InteractOnServer`))))

(event `InteractOnServer`
  (bind _output_get (set `self.InteractToggle` (not (`self.InteractToggle`))))
  (`KismetSystemLibrary.PrintString` (`KismetStringLibrary.Conv_BoolToString` _output_get)))

(event `self.Sphere.OnComponentBeginOverlap`
  (params (OverlappedComponent :type "PrimitiveComponent Object Reference") (OtherActor :type "Actor Object Reference") (OtherComp :type "PrimitiveComponent Object Reference") (OtherBodyIndex :type Integer) (bFromSweep :type Boolean) (SweepResult :type "HitResult Structure (by ref)"))
  (bind _returnvalue (`self.GetComponentByClass` OtherActor "/Game/Inventory/AC_Inventory.AC_Inventory_C"))
  ;[1 1 1] Пересечение коллизиии сферы позволяет подобрать предмет и пихнуть в инвентарь, после чего предмет уничтожается в мире
  (`/Engine/EditorBlueprintResources/StandardMacros.IsValid` _returnvalue
    (:`Is Valid`
      (bind _returnvalue_2 (`/Game/Inventory/AC_Inventory.PickUpItem` _returnvalue self))
      (if _returnvalue_2
        (`self.K2_DestroyActor`)))))

(fn `GetInteractionWidgetRef`
  (returns (Ref :type "WidgetComponent Object Reference"))
  ;[1 1 1] Добавление функции и виджета с которой она будет работать
  (return (`self.Widget`)))

(fn `OnRep_InteractToggle`
  (bind _returnvalue (`self.GetComponentByClass` (`GameplayStatics.GetPlayerCameraManager` 0) "/Game/Inventory/AC_Inventory.AC_Inventory_C"))
  (if (`self.InteractToggle`)
    (`/Engine/EditorBlueprintResources/StandardMacros.IsValid` _returnvalue
      (:`Is Valid`
        (bind _returnvalue_2 (`/Game/Inventory/AC_Inventory.PickUpItem` _returnvalue self))
        (if _returnvalue_2
          (`self.K2_DestroyActor`)))
      (:`Is Not Valid`
        (`KismetSystemLibrary.PrintString` "is not valid" true true (struct :`R` 1.0 :`G` 0.127908 :`A` 1.0))))))

(fn `UserConstructionScript`)