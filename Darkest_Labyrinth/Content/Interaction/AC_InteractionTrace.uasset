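; Player interaction component that detects the BP_InteractionArea under the camera and triggers it on input.
; Each tick, a Visibility line trace from player camera 0 tracks the hit actor, toggling area focus when it changes.
; TryToInteract fires only for zero-or-negative-duration areas; timed holds have no logic here.
; InteractOnServer forwards the interaction to the area's parent actor through an interface message, decoupling it from concrete interactables.
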(event `self.ReceiveTick`
  (params (DeltaSeconds :type "Float (single-precision)"))
  ;[1 1 1] Вызов функции Trace, каждый тик
  (`self.Trace`))

(event `TryToInteract`
  (params (In :type Boolean))
  ;[1 1 1] Ивент, срабатываемый при нажатии на Е
  ;[1 1 1] Нажали на Е?
  (if In
    ;[1 1 1] Трэйсинг в интеракт объект?
    (if (`self.IsTracingInteractionArea`)
      ;[1 1 1] Беру длительность нажатия на интеракт объект
      (bind _output_get (set `self.Interact Duraton` (`/Game/Interaction/InteractionArea/BP_InteractionArea.InteractDuraton` (`self.FocusedInteractionArea`))))
      ;[1 1 1] Длительность больше 0?
      (if (not (> _output_get 0.0))
        ;[0.1195 0.9131 1] Вызов функции Interact On Server и передача значения Focused Area в ивент
        (`self.InteractOnServer` (`self.FocusedInteractionArea`))))))

(event `InteractOnServer`
  (params (InteractionArea :type "/Game/Interaction/InteractionArea/BP_InteractionArea Object Reference"))
  ;[0.1195 0.9131 1] Передача Interaction Area на котором Focused. Получение его родителя. Вызов функции Interface Interact с целевым родителем
  (message `/Game/Interaction/BI_Interaction.InterfaceInteract` (`Actor.GetParentActor` InteractionArea)))

(fn `Trace`
  (bind _returnvalue (`GameplayStatics.GetPlayerCameraManager` 0))
  (bind _returnvalue_2 (`Actor.K2_GetActorLocation` _returnvalue))
  ;[1 1 1] Старт функции Trace
  ;[1 1 1] Получаю стартовую и конечную точку трейса
  (bind (_outhit _returnvalue_3) (`KismetSystemLibrary.LineTraceSingle` _returnvalue_2 (+ _returnvalue_2 (* (`KismetMathLibrary.GetForwardVector` (`Actor.K2_GetActorRotation` _returnvalue)) (`self.Length`))) "TraceTypeQuery1"))
  ;[1 1 1] Есть столкновение?
  (if _returnvalue_3
    (bind (_bblockinghit _binitialoverlap _time _distance _location _impactpoint _normal _impactnormal _physmat _hitactor) (`GameplayStatics.BreakHitResult` _outhit))
    ;[1 1 1] Актор в фокусе и игрок - не одно и тоже?
    (if (!= (`self.FocusedActor`) _hitactor)
      (set `self.FocusedActor` _hitactor)
      (`self.TraceInteractionArea` (== (`GameplayStatics.GetObjectClass` _hitactor) "/Game/Interaction/InteractionArea/BP_InteractionArea.BP_InteractionArea_C")))
    (else
      ;[1 1 1] Функция Interaction Area не срабатывает
      (`self.TraceInteractionArea` false))))

(fn `TraceInteractionArea`
  (params (Trace :type Boolean))
  ;[1 1 1] Функция с переданным значением Trace
  ;[1 1 1] Трейс на BP?
  (if Trace
    ;[1 1 1] Попали в Interaction Area?
    (if (`self.IsTracingInteractionArea`)
      (`/Game/Interaction/InteractionArea/BP_InteractionArea.ToggleFocus` (`self.FocusedInteractionArea`) false))
    (bind _asbp_interaction_area (cast `/Game/Interaction/InteractionArea/BP_InteractionArea` (`self.FocusedActor`)))
    (bind _output_get (set `self.FocusedInteractionArea` _asbp_interaction_area))
    (`/Game/Interaction/InteractionArea/BP_InteractionArea.ToggleFocus` _output_get true)
    (set `self.IsTracingInteractionArea` true)
    (else
      ;[1 1 1] Ранее попали в Interaction Area?
      (if (`self.IsTracingInteractionArea`)
        ;[1 1 1] Установка значения Inter Area = 0; Вызов Toggle Focus, установка значения Focused для F Inter Area = 0
        (set `self.IsTracingInteractionArea` false)
        (`/Game/Interaction/InteractionArea/BP_InteractionArea.ToggleFocus` (`self.FocusedInteractionArea`) false)
        (set `self.FocusedActor` null)
        (set `self.FocusedInteractionArea` null)))))