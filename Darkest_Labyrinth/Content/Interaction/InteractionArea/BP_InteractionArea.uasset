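; BP_InteractionArea is an interaction area actor that relays focus changes to its parent actor and shows or hides that actor's interaction widget.
; ToggleFocus stores the Focused state, prints a debug message and forwards the state through an interface message.
; It fetches the parent's widget reference by message and, if the parent is valid, sets the widget's visibility to match focus, otherwise printing the failed check.
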(event `ToggleFocus`
  (params (Focused :type Boolean))
  (bind _returnvalue (`self.GetParentActor`))
  (bind _returnvalue_2 (`KismetSystemLibrary.IsValid` _returnvalue))
  ;[1 1 1] Ивент фокусировки на нашем BP с установкой значения focused == True, когда ивент активирован
  (set `self.Focused` Focused)
  (`KismetSystemLibrary.PrintString` "Я В ФОКУСЕ" true true (struct :`R` 1.0 :`B` 0.2406 :`A` 1.0))
  (message `/Game/Interaction/BI_Interaction.Interface_ToggleFocus` (`self.GetParentActor`) (`self.Focused`))
  (bind _ref (message `/Game/Interaction/BI_Interaction.GetInteractionWidgetRef` _returnvalue))
  (if _returnvalue_2
    (`SceneComponent.SetHiddenInGame` _ref (not (`self.Focused`)) false)
    (else
      (`KismetSystemLibrary.PrintString` (`KismetStringLibrary.Conv_BoolToString` _returnvalue_2)))))

(fn `UserConstructionScript`)