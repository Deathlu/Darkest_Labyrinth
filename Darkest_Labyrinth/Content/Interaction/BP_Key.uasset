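; BP_Key is an interactable key that flies toward the player's camera when used.
; It handles interaction-interface events, printing focus changes as debug text and exposing its widget through a getter.
; Interacting calls InteractOnServer to flip InteractToggle, whose OnRep is empty, while a Timeline lerps the actor from its current location toward player 0's camera.
; Each Timeline update also requests a short Delay before setting the Key component visible.
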(event `/Game/Interaction/BI_Interaction.Interface_ToggleFocus`
  (params (Focus :type Boolean))
  (`KismetSystemLibrary.PrintText` (`KismetTextLibrary.Conv_BoolToText` Focus) true true (struct :`R` 0.842565 :`G` 0.199542 :`B` 1.0 :`A` 1.0)))

(event `/Game/Interaction/BI_Interaction.InterfaceInteract`
  (`self.Interact On Server`)
  (bind (_direction _newtrack_1) (`Timeline|Timeline` :!via `PlayFromStart`)
    (:`Update`
      (`self.K2_SetActorLocation` (`KismetMathLibrary.VLerp` (`self.K2_GetActorLocation`) (`self.K2_GetActorLocation` (`GameplayStatics.GetPlayerCameraManager` 0)) _newtrack_1))
      (`KismetSystemLibrary.Delay` 0.2)
      (`SceneComponent.SetHiddenInGame` (`self.Key`) false false))))

(event `Interact On Server`
  (set `self.InteractToggle` (not (`self.InteractToggle`))))

(fn `GetInteractionWidgetRef`
  (returns (Ref :type "WidgetComponent Object Reference"))
  ;[1 1 1] Добавление функции и виджета с которой она будет работать
  (return (`self.Widget`)))

(fn `OnRep_InteractToggle`)

(fn `UserConstructionScript`)