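; BP_MonsterCharacter_4 is an AI monster character that writes what it perceives into its behavior tree blackboard.
; Perception of the third-person player character updates a seen-player flag.
; The Escape event flags that the monster was lit and sets a hard-coded escape coordinate; no connected logic clears that flag.
; Helper functions supply a fixed ideal range and map a speed state to max walk speed, switched from BTT_SetMovementSpeed.
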(event `self.AIPerception.OnTargetPerceptionUpdated`
  (params (Actor :type "Actor Object Reference") (Stimulus :type "AIStimulus Structure"))
  (cast `/Game/ThirdPerson/Blueprints/BP_ThirdPersonCharacter` Actor)
  (`BlackboardComponent.SetValueAsBool` (`AIBlueprintHelperLibrary.GetBlackboard` (`AIBlueprintHelperLibrary.GetAIController` self)) "hasSeenPlayer?" (`.bSuccessfullySensed` (break `AIStimulus` Stimulus))))

(event `/Game/AI/BPI_Escape.Escape`
  (`KismetSystemLibrary.PrintString` "HasLighted!")
  (`BlackboardComponent.SetValueAsBool` (`AIBlueprintHelperLibrary.GetBlackboard` (`AIBlueprintHelperLibrary.GetAIController` self)) "hasLighted?" true)
  (`BlackboardComponent.SetValueAsVector` (`AIBlueprintHelperLibrary.GetBlackboard` (`AIBlueprintHelperLibrary.GetAIController` self)) "EscapeCoord" (1610.0 1780.0 0.0)))

(fn `GetIdealRange`
  (returns (IdealRange :type "Float (double-precision)"))
  (return 350.0))

(fn `SetMovementSpeed`
  (params (Speed :type "/Game/AI/E_MovementSpeed Enum" :default "NewEnumerator0"))
  (returns (SpeedValue :type "Float (double-precision)"))
  ;[1 1 1] Выставляем варианты скорости, которые переключаются уже в BTT_SetMovementSpeed
  (set `CharacterMovementComponent.MaxWalkSpeed` (select `/Game/AI/E_MovementSpeed` Speed :`NewEnumerator1` 200.0 :`NewEnumerator2` 400.0 :`NewEnumerator3` 150.0 :!type "Float (single-precision)") (`self.CharacterMovement`))
  (return 0.0))

(fn `UserConstructionScript`)