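; BP_Monster is an AI monster that wanders on its own, steering away from obstacles with a simple forward probe.
; Each tick it runs a debug-drawn Visibility multi-line trace along its forward vector for Length units.
; While that trace reports a blocking hit, it rotates its stored Direction by a small fixed step per frame, so turn speed depends on frame rate.
; It always feeds Direction into movement input at half scale.
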(event `self.ReceiveTick`
  (params (DeltaSeconds :type "Float (single-precision)"))
  (bind _returnvalue (`self.K2_GetActorLocation`))
  (bind (_outhits _returnvalue_2) (`KismetSystemLibrary.LineTraceMulti` :`Start` _returnvalue :`End` (+ _returnvalue (* (`self.GetActorForwardVector`) (`self.length`))) :`TraceChannel` "TraceTypeQuery1" :`DrawDebugType` "ForOneFrame"))
  (if _returnvalue_2
    (set `self.Direction` (`KismetMathLibrary.GreaterGreater_VectorRotator` (`self.Direction`) (struct :`Yaw` 1.0))))
  (`self.AddMovementInput` (`self.Direction`) 0.5))

(fn `UserConstructionScript`)