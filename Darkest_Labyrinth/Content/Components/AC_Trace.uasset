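; Actor component that casts a debug trace along the player camera's view, apparently standing in for a lantern's light beam.
; LightOnOff takes the lantern's active state, sets the beam length to a fixed reach or zero, then runs a multi capsule trace on Visibility from the camera.
; Both branches print a debug string, and the trace hits are unused.
; The event graph holds only disabled events and an unconnected copy of the trace.
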(fn `LightOn/Off`
  (params (`CLanternActive?` :type Boolean))
  (bind _returnvalue (`GameplayStatics.GetPlayerCameraManager` 0))
  (bind _returnvalue_2 (`GameplayStatics.GetPlayerCameraManager` 0))
  (bind _returnvalue_3 (`Actor.K2_GetActorLocation` _returnvalue))
  (bind _returnvalue_4 (`Actor.K2_GetActorLocation` _returnvalue_2))
  (if `CLanternActive?`
    (bind _output_get (set `self.LightLength` 400.0))
    (`KismetSystemLibrary.PrintString` "Vector Light 2")
    (`KismetSystemLibrary.CapsuleTraceMulti` :`Start` _returnvalue_3 :`End` (+ (* (`KismetMathLibrary.GetForwardVector` (`Actor.K2_GetActorRotation` _returnvalue)) _output_get) _returnvalue_3) :`TraceChannel` "TraceTypeQuery1" :`DrawDebugType` "ForDuration")
    (else
      (bind _output_get_2 (set `self.LightLength` 0.0))
      (`KismetSystemLibrary.PrintString` "Vector Light 2")
      (`KismetSystemLibrary.CapsuleTraceMulti` :`Start` _returnvalue_4 :`End` (+ (* (`KismetMathLibrary.GetForwardVector` (`Actor.K2_GetActorRotation` _returnvalue_2)) _output_get_2) _returnvalue_4) :`TraceChannel` "TraceTypeQuery1" :`DrawDebugType` "ForDuration"))))