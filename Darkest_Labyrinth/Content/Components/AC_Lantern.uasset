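; Lantern component that toggles the crystal light on the character's lantern.
; CristalLantOnOff requires a held lantern and loaded crystal, otherwise printing a message, then flips the light's visibility and CLanternActive.
; It also sets the lantern mesh's glass material, using the glow version only when the crystal switches off while LanternActive is true.
; BeginPlay and Tick are empty, and NewMacro holds unused camera-forward point math.
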(fn `CristalLantOnOff`
  (if (`self.HasLantern?`)
    (if (`self.LanternActive?`)
      (if (`self.CristalLoad?`)
        (if (`self.CLanternActive?`)
          (`SceneComponent.SetVisibility` (`/Game/Characters/ThirdPerson/Blueprints/BP_ThirdPersonCharacter.CristalLight` (`self.Character`)) false false)
          (set `self.CLanternActive?` false)
          (`PrimitiveComponent.SetMaterial` (`/Game/Characters/ThirdPerson/Blueprints/BP_ThirdPersonCharacter.SM_Lantern_Full` (`self.Character`)) 1 "/Game/FlashLight/Mesh/M_LanternGlass_Glow.M_LanternGlass_Glow")
          (else
            (`SceneComponent.SetVisibility` (`/Game/Characters/ThirdPerson/Blueprints/BP_ThirdPersonCharacter.CristalLight` (`self.Character`)) true false)
            (set `self.CLanternActive?` true)
            (`PrimitiveComponent.SetMaterial` (`/Game/Characters/ThirdPerson/Blueprints/BP_ThirdPersonCharacter.SM_Lantern_Full` (`self.Character`)) 1 "/Game/FlashLight/Mesh/MI_lantern_glass.MI_lantern_glass")))
        (else
          (`KismetSystemLibrary.PrintString` "No Cristal!")))
      (elif (`self.CristalLoad?`)
        (if (`self.CLanternActive?`)
          (`SceneComponent.SetVisibility` (`/Game/Characters/ThirdPerson/Blueprints/BP_ThirdPersonCharacter.CristalLight` (`self.Character`)) false false)
          (set `self.CLanternActive?` false)
          (`PrimitiveComponent.SetMaterial` (`/Game/Characters/ThirdPerson/Blueprints/BP_ThirdPersonCharacter.SM_Lantern_Full` (`self.Character`)) 1 "/Game/FlashLight/Mesh/MI_lantern_glass.MI_lantern_glass")
          (else
            (`SceneComponent.SetVisibility` (`/Game/Characters/ThirdPerson/Blueprints/BP_ThirdPersonCharacter.CristalLight` (`self.Character`)) true false)
            (set `self.CLanternActive?` true)
            (`PrimitiveComponent.SetMaterial` (`/Game/Characters/ThirdPerson/Blueprints/BP_ThirdPersonCharacter.SM_Lantern_Full` (`self.Character`)) 1 "/Game/FlashLight/Mesh/MI_lantern_glass.MI_lantern_glass")))
        (else
          (`KismetSystemLibrary.PrintString` "No Cristal! 2"))))
    (else
      (`KismetSystemLibrary.PrintString` "No Lantern"))))