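; AC_LightTrace is a component that detects whether the player's light, cast along the camera view, hits a monster.
; LightOnOff runs a debug-drawn Visibility line trace from the camera, tracks FocusedActor, and passes LightedMonster whether a newly hit actor is BP_MonsterCharacter_4, or false on a miss.
; LightedMonster is empty here, the off branch is unreachable behind a constant true, and the EventGraph's capsule trace is unconnected.
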(fn `LightedMonster`
  (params (Trace :type Boolean)))

(fn `LightOn/Off`
  (bind _returnvalue (`GameplayStatics.GetPlayerCameraManager` 0))
  (bind _returnvalue_2 (`Actor.K2_GetActorLocation` _returnvalue))
  (`KismetSystemLibrary.PrintString` "HI LITGHT")
  (if true
    (bind _output_get (set `self.LightLength` 400.0))
    (`KismetSystemLibrary.PrintString` "Vector Light 2")
    (bind (_outhit _returnvalue_3) (`KismetSystemLibrary.LineTraceSingle` :`Start` _returnvalue_2 :`End` (+ _returnvalue_2 (* (`KismetMathLibrary.GetForwardVector` (`Actor.K2_GetActorRotation` _returnvalue)) _output_get)) :`TraceChannel` "TraceTypeQuery1" :`DrawDebugType` "ForDuration"))
    (if _returnvalue_3
      (bind (_bblockinghit _binitialoverlap _time _distance _location _impactpoint _normal _impactnormal _physmat _hitactor) (`GameplayStatics.BreakHitResult` _outhit))
      (if (!= (`self.FocusedActor`) _hitactor)
        (set `self.FocusedActor` _hitactor)
        (`self.LightedMonster` (== (`GameplayStatics.GetObjectClass` _hitactor) "/Game/AI/BP_MonsterCharacter_4.BP_MonsterCharacter_4_C")))
      (else
        (`self.LightedMonster` false)))
    (else
      (bind _output_get_2 (set `self.LightLength` 0.0))
      (`KismetSystemLibrary.PrintString` "Vector Light 2")
      (bind (_outputpin _returnvalue_4) (`self.LengthCalculate` _output_get_2))
      (`KismetSystemLibrary.LineTraceSingle` :`Start` _outputpin :`End` _returnvalue_4 :`TraceChannel` "TraceTypeQuery1" :`DrawDebugType` "ForDuration"))))